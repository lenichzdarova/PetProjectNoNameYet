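; BP_PlayerCharacter is the player-controlled character Blueprint, providing basic axis-driven movement and look controls.
; The four input axis events pass their values to matching functions for forward and sideways movement, pitch and yaw.
; Movement directions derive only from the control rotation's yaw, so travel follows the camera heading and stays horizontal regardless of pitch.
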(event `InputAxis|MoveForward`
  (params (AxisValue :type "Float (single-precision)"))
  (`self.MoveForward` AxisValue))

(event `InputAxis|MoveRight`
  (params (AxisValue :type "Float (single-precision)"))
  (`self.MoveRight` AxisValue))

(event `InputAxis|LookUp`
  (params (AxisValue :type "Float (single-precision)"))
  (`self.LookUp` AxisValue))

(event `InputAxis|LookRight`
  (params (AxisValue :type "Float (single-precision)"))
  (`self.Look RIght` AxisValue))

(fn `Look RIght`
  (params (InputValue :type "Float (double-precision)"))
  (`self.AddControllerYawInput` InputValue))

(fn `LookUp`
  (params (InputValue :type "Float (double-precision)"))
  (`self.AddControllerPitchInput` InputValue))

(fn `MoveForward`
  (params (AxisValue :type "Float (double-precision)"))
  (bind (_returnvalue_roll _returnvalue_pitch _returnvalue_yaw) (`KismetMathLibrary.BreakRotator` (`self.GetControlRotation`)))
  (`self.AddMovementInput` (`KismetMathLibrary.GetForwardVector` (`KismetMathLibrary.MakeRotator` 0.0 0.0 _returnvalue_yaw)) AxisValue))

(fn `MoveRight`
  (params (InputValue :type "Float (double-precision)"))
  (bind (_returnvalue_roll _returnvalue_pitch _returnvalue_yaw) (`KismetMathLibrary.BreakRotator` (`self.GetControlRotation`)))
  (`self.AddMovementInput` (`KismetMathLibrary.GetRightVector` (`KismetMathLibrary.MakeRotator` 0.0 0.0 _returnvalue_yaw)) InputValue))

(fn `UserConstructionScript`)