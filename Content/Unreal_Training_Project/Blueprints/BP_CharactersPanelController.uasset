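; BP_CharactersPanelController links a party object to a characters panel widget and handles hotkey selection of the active character.
; Initialize stores both references, subscribes to the party-changed event and builds the widget's buttons from the party members, which OnPartyChanged rebuilds.
; Five Enhanced Input actions, IA_1 through IA_5, pass a slot index to the party's SetActiveCharacter.
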(event `EnhancedInput|/Game/Unreal_Training_Project/Blueprints/Inputs/IA_1`
  (params (ActionValue :type Boolean) (ElapsedSeconds :type "Float (double-precision)") (TriggeredSeconds :type "Float (double-precision)") (InputAction :type "InputAction Object Reference" :default "/Game/Unreal_Training_Project/Blueprints/Inputs/IA_1.IA_1"))
  (:`Triggered`
    (`self.OnSelectCharacter` 0)))

(event `EnhancedInput|/Game/Unreal_Training_Project/Blueprints/Inputs/IA_2`
  (params (ActionValue :type Boolean) (ElapsedSeconds :type "Float (double-precision)") (TriggeredSeconds :type "Float (double-precision)") (InputAction :type "InputAction Object Reference" :default "/Game/Unreal_Training_Project/Blueprints/Inputs/IA_2.IA_2"))
  (:`Triggered`
    (`self.OnSelectCharacter` 1)))

(event `EnhancedInput|/Game/Unreal_Training_Project/Blueprints/Inputs/IA_3`
  (params (ActionValue :type Boolean) (ElapsedSeconds :type "Float (double-precision)") (TriggeredSeconds :type "Float (double-precision)") (InputAction :type "InputAction Object Reference" :default "/Game/Unreal_Training_Project/Blueprints/Inputs/IA_3.IA_3"))
  (:`Triggered`
    (`self.OnSelectCharacter` 2)))

(event `EnhancedInput|/Game/Unreal_Training_Project/Blueprints/Inputs/IA_4`
  (params (ActionValue :type Boolean) (ElapsedSeconds :type "Float (double-precision)") (TriggeredSeconds :type "Float (double-precision)") (InputAction :type "InputAction Object Reference" :default "/Game/Unreal_Training_Project/Blueprints/Inputs/IA_4.IA_4"))
  (:`Triggered`
    (`self.OnSelectCharacter` 3)))

(event `EnhancedInput|/Game/Unreal_Training_Project/Blueprints/Inputs/IA_5`
  (params (ActionValue :type Boolean) (ElapsedSeconds :type "Float (double-precision)") (TriggeredSeconds :type "Float (double-precision)") (InputAction :type "InputAction Object Reference" :default "/Game/Unreal_Training_Project/Blueprints/Inputs/IA_5.IA_5"))
  (:`Triggered`
    (`self.OnSelectCharacter` 4)))

(fn `BindEvents`
  (add `/Game/Unreal_Training_Project/Blueprints/RPG_System/BP_PlayerParty.PartyChanged` (`self.party`) (`|CreateDelegate` :!event `OnPartyChanged`)))

(fn `Initialize`
  (params (widget :type "/Game/Unreal_Training_Project/Blueprints/UI/UI_CharactersPanel Object Reference") (Party :type "/Game/Unreal_Training_Project/Blueprints/RPG_System/BP_PlayerParty Object Reference"))
  (set `self.widget` widget)
  (bind _output_get (set `self.party` Party))
  (`self.BindEvents`)
  (bind _newparam (`/Game/Unreal_Training_Project/Blueprints/RPG_System/BP_PlayerParty.GetPartyMembers` _output_get))
  (`/Game/Unreal_Training_Project/Blueprints/UI/UI_CharactersPanel.InitializeButtons` (`self.widget`) _newparam))

(fn `OnPartyChanged`
  (bind _newparam (`/Game/Unreal_Training_Project/Blueprints/RPG_System/BP_PlayerParty.GetPartyMembers` (`self.party`)))
  (`/Game/Unreal_Training_Project/Blueprints/UI/UI_CharactersPanel.InitializeButtons` (`self.widget`) _newparam))

(fn `OnSelectCharacter`
  (params (Index :type Integer))
  (`/Game/Unreal_Training_Project/Blueprints/RPG_System/BP_PlayerParty.SetActiveCharacter` (`self.party`) Index))