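; First-person player Blueprint with Enhanced Input movement, jump and a visible mouse cursor for interaction, apparently for a party-based RPG prototype.
; Holding the look toggle hides and recenters the cursor to enable camera look.
; BeginPlay builds a test party of BP_Character objects and shows its characters panel.
; The action input only debug-traces under the cursor; spellbook input opens its widget, while spell selection merely fetches the active character's spell.
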(event `self.ReceiveBeginPlay`
  (bind _asplayer_controller (cast `PlayerController` (`self.GetController`)))
  (message `EnhancedInputSubsystemInterface.AddMappingContext` (pcsubsystem `EnhancedInputLocalPlayerSubsystem` _asplayer_controller) "/Game/Unreal_Training_Project/Blueprints/Inputs/IAM_FirstPerson.IAM_FirstPerson" 0 (struct))
  (set `PlayerController.bShowMouseCursor` true (`GameplayStatics.GetPlayerController` 0))
  (`WidgetBlueprintLibrary.SetInputMode_GameAndUIEx` _asplayer_controller null "LockAlways")
  (`self.CreateTestParty`))

(event `EnhancedInput|/Game/Unreal_Training_Project/Blueprints/Inputs/IA_Action`
  (params (ActionValue :type Boolean) (ElapsedSeconds :type "Float (double-precision)") (TriggeredSeconds :type "Float (double-precision)") (InputAction :type "InputAction Object Reference" :default "/Game/Unreal_Training_Project/Blueprints/Inputs/IA_Action.IA_Action"))
  (bind (_worldlocation _worlddirection) (`PlayerController.DeprojectMousePositionToWorld` (`GameplayStatics.GetPlayerController` 0)))
  (:`Triggered`
    (`KismetSystemLibrary.LineTraceSingle` :`Start` _worldlocation :`End` (+ _worldlocation (* _worlddirection 1000)) :`TraceChannel` "TraceTypeQuery1" :`DrawDebugType` "ForOneFrame")))

(event `EnhancedInput|/Game/Unreal_Training_Project/Blueprints/Inputs/IA_Spellbook`
  (params (ActionValue :type Boolean) (ElapsedSeconds :type "Float (double-precision)") (TriggeredSeconds :type "Float (double-precision)") (InputAction :type "InputAction Object Reference" :default "/Game/Unreal_Training_Project/Blueprints/Inputs/IA_Spellbook.IA_Spellbook"))
  (:`Triggered`
    (`self.OpenSpellbook`)))

(event `EnhancedInput|/Game/Unreal_Training_Project/Blueprints/Inputs/IA_LookToggle`
  (params (ActionValue :type Boolean) (ElapsedSeconds :type "Float (double-precision)") (TriggeredSeconds :type "Float (double-precision)") (InputAction :type "InputAction Object Reference" :default "/Game/Unreal_Training_Project/Blueprints/Inputs/IA_LookToggle.IA_LookToggle"))
  (bind _returnvalue (`GameplayStatics.GetPlayerController` 0))
  (bind (_sizex _sizey) (`PlayerController.GetViewportSize` _returnvalue))
  (:`Triggered`
    (set `PlayerController.bShowMouseCursor` false _returnvalue)
    (`PlayerController.SetMouseLocation` _returnvalue (/ _sizex 2) (/ _sizey 2) :!label _label))
  (:`Completed`
    (set `PlayerController.bShowMouseCursor` true _returnvalue)
    (goto _label)))

(event `EnhancedInput|/Game/Unreal_Training_Project/Blueprints/Inputs/IA_Look`
  (params (ActionValue :type "Vector2D Structure") (ElapsedSeconds :type "Float (double-precision)") (TriggeredSeconds :type "Float (double-precision)") (InputAction :type "InputAction Object Reference" :default "/Game/Unreal_Training_Project/Blueprints/Inputs/IA_Look.IA_Look"))
  (:`Triggered`
    (if (`|GetInputActionValue`)
      (`self.Look` (`KismetMathLibrary.MakeVector2D` ActionValue_X ActionValue_Y)))))

(event `EnhancedInput|/Game/Unreal_Training_Project/Blueprints/Inputs/IA_Move`
  (params (ActionValue :type "Vector2D Structure") (ElapsedSeconds :type "Float (double-precision)") (TriggeredSeconds :type "Float (double-precision)") (InputAction :type "InputAction Object Reference" :default "/Game/Unreal_Training_Project/Blueprints/Inputs/IA_Move.IA_Move"))
  (:`Triggered`
    (`self.Move` (`KismetMathLibrary.MakeVector2D` ActionValue_X ActionValue_Y))))

(event `EnhancedInput|/Game/Unreal_Training_Project/Blueprints/Inputs/IA_Jump`
  (params (ActionValue :type Boolean) (ElapsedSeconds :type "Float (double-precision)") (TriggeredSeconds :type "Float (double-precision)") (InputAction :type "InputAction Object Reference" :default "/Game/Unreal_Training_Project/Blueprints/Inputs/IA_Jump.IA_Jump"))
  (:`Triggered`
    (`self.Jump`)))

(fn `CreateTestParty`
  (bind _returnvalue (`|GenericCreateObject` "/Game/Unreal_Training_Project/Blueprints/RPG_System/BP_PlayerParty.BP_PlayerParty_C"))
  (bind _output_get (set `self.playerParty` _returnvalue))
  (`/Game/Unreal_Training_Project/Blueprints/RPG_System/BP_PlayerParty.Initialize` _output_get)
  (for _ (range 4)
    (bind _returnvalue_2 (`|GenericCreateObject` "/Game/Unreal_Training_Project/Blueprints/RPG_System/BP_Character.BP_Character_C"))
    (`/Game/Unreal_Training_Project/Blueprints/RPG_System/BP_Character.Initialize` _returnvalue_2)
    (`/Game/Unreal_Training_Project/Blueprints/RPG_System/BP_PlayerParty.AddCharacter` (`self.playerParty`) _returnvalue_2))
  (bind _returnvalue_3 (`|CreateWidget` "/Game/Unreal_Training_Project/Blueprints/UI/CharactersPanel/UI_CharactersPanel.UI_CharactersPanel_C"))
  (`/Game/Unreal_Training_Project/Blueprints/UI/CharactersPanel/UI_CharactersPanel.Initialize` _returnvalue_3 _returnvalue)
  (`UserWidget.AddToViewport` _returnvalue_3 0))

(fn `Look`
  (params (InputValue :type "Vector2D Structure"))
  (bind (_returnvalue_roll _returnvalue_pitch _returnvalue_yaw) (`KismetMathLibrary.BreakRotator` (`SceneComponent.K2_GetComponentRotation` (`self.Camera`))))
  (`self.AddControllerYawInput` InputValue_X)
  (`SceneComponent.K2_SetWorldRotation` (`self.Camera`) (`KismetMathLibrary.MakeRotator` 0.0 (+ InputValue_Y _returnvalue_pitch) _returnvalue_yaw) false false))

(fn `Move`
  (params (InputValue :type "Vector2D Structure"))
  (locals (NewLocalVar :type Boolean))
  (bind _returnvalue (`self.GetControlRotation`))
  (`self.AddMovementInput` (`KismetMathLibrary.GetForwardVector` _returnvalue) InputValue_X)
  (`self.AddMovementInput` (`KismetMathLibrary.GetRightVector` _returnvalue) InputValue_Y))

(fn `OnSpellSelected`
  (params (SpellIndex :type Integer))
  (bind _character (`/Game/Unreal_Training_Project/Blueprints/RPG_System/BP_PlayerParty.GetActiveCharacter` (`self.playerParty`)))
  (`/Game/Unreal_Training_Project/Blueprints/RPG_System/BP_Spellbook.GetSpell` (`/Game/Unreal_Training_Project/Blueprints/RPG_System/BP_Character.Spellbook` _character) SpellIndex))

(fn `OpenSpellbook`
  (bind _returnvalue (`|CreateWidget` "/Game/Unreal_Training_Project/Blueprints/UI/Spellbook/UI_Spellbook.UI_Spellbook_C"))
  (`UserWidget.AddToViewport` _returnvalue 0))

(fn `UserConstructionScript`)