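; BP_AbilitiesHandler is an RPG component that turns the six ability scores (Strength through Charisma) into bonuses.
; Initialize stores a FeatsHandler reference, which the shown graphs never use.
; Each getter reads its score from a FinalValue struct and passes it to a shared AbilityBonusCalculator, which applies the D&D-style (score − 10) / 2 formula.
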(fn `AbilityBonusCalculator`
  (params (abilityValue :type Integer))
  (returns (bonusValue :type Integer))
  (return (/ (- abilityValue 10) 2)))

(fn `GetCharisma`
  (returns (charismaBonus :type Integer))
  (bind (_finalvalue_strength _finalvalue_constitution _finalvalue_dexterity _finalvalue_intelligence _finalvalue_wisdom _finalvalue_charisma) (break `/Game/Unreal_Training_Project/Blueprints/RPG_System/Abilities` (`self.finalValue`)))
  (bind _bonusvalue (`self.AbilityBonusCalculator` _finalvalue_charisma))
  (return _bonusvalue))

(fn `GetConstitutionBonus`
  (returns (constiitutionBonus :type Integer))
  (bind (_finalvalue_strength _finalvalue_constitution) (break `/Game/Unreal_Training_Project/Blueprints/RPG_System/Abilities` (`self.finalValue`)))
  (bind _bonusvalue (`self.AbilityBonusCalculator` _finalvalue_constitution))
  (return _bonusvalue))

(fn `GetDexterityBonus`
  (returns (dexterityBonus :type Integer))
  (bind (_finalvalue_strength _finalvalue_constitution _finalvalue_dexterity) (break `/Game/Unreal_Training_Project/Blueprints/RPG_System/Abilities` (`self.finalValue`)))
  (bind _bonusvalue (`self.AbilityBonusCalculator` _finalvalue_dexterity))
  (return _bonusvalue))

(fn `GetIntelligenceBonus`
  (returns (intelligenceBonus :type Integer))
  (bind (_finalvalue_strength _finalvalue_constitution _finalvalue_dexterity _finalvalue_intelligence) (break `/Game/Unreal_Training_Project/Blueprints/RPG_System/Abilities` (`self.finalValue`)))
  (bind _bonusvalue (`self.AbilityBonusCalculator` _finalvalue_intelligence))
  (return _bonusvalue))

(fn `GetStrengthBonus`
  (returns (strengthBonus :type Integer))
  (bind _finalvalue_strength (break `/Game/Unreal_Training_Project/Blueprints/RPG_System/Abilities` (`self.finalValue`)))
  (bind _bonusvalue (`self.AbilityBonusCalculator` _finalvalue_strength))
  (return _bonusvalue))

(fn `GetWisdomBonus`
  (returns (wisdomValue :type Integer))
  (bind (_finalvalue_strength _finalvalue_constitution _finalvalue_dexterity _finalvalue_intelligence _finalvalue_wisdom) (break `/Game/Unreal_Training_Project/Blueprints/RPG_System/Abilities` (`self.finalValue`)))
  (bind _bonusvalue (`self.AbilityBonusCalculator` _finalvalue_wisdom))
  (return _bonusvalue))

(fn `Initialize`
  (params (featsHandler :type "/Game/Unreal_Training_Project/Blueprints/RPG_System/BP_FeatsHandler Object Reference"))
  (set `self.featsHandler` featsHandler))