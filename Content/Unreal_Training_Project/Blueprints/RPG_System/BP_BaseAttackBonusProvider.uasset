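; BP_BaseAttackBonusProvider computes an RPG character's base attack bonus from profession and experience level.
; GetAttackBonus multiplies the level by a per-profession progression rate and floors the result.
; DefineProgressionValue selects that rate from shared constants: high for Fighter and Paladin, medium for Rogue, low for Mage.
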(fn `DefineProgressionValue`
  (params (profession :type "/Game/Unreal_Training_Project/Blueprints/RPG_System/Enums/ProfessionEnum Enum" :default "NewEnumerator0"))
  (returns (progressionValue :type "Float (double-precision)"))
  (locals (result :type "Float (double-precision)"))
  (switch `/Game/Unreal_Training_Project/Blueprints/RPG_System/Enums/ProfessionEnum` profession
    (:`NewEnumerator0`
      (set `local.result` (`self.HightProgressionConst`)))
    (:`NewEnumerator1`
      (set `local.result` (`self.LowProgressionConst`)))
    (:`NewEnumerator2`
      (set `local.result` (`self.MediumProgressionConst`)))
    (:`NewEnumerator3`
      (set `local.result` (`self.HightProgressionConst`))))
  (return (`local.result`)))

(fn `GetAttackBonus`
  (params (profession :type "/Game/Unreal_Training_Project/Blueprints/RPG_System/Enums/ProfessionEnum Enum" :default "NewEnumerator0") (experienceLevel :type Integer))
  (returns (attackBonus :type Integer))
  (locals (result :type Integer))
  (bind _progressionvalue (`self.DefineProgressionValue` profession))
  (bind _output_get (set `local.result` (`KismetMathLibrary.FFloor` (* experienceLevel _progressionvalue))))
  (return _output_get))