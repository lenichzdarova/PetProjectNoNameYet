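; BP_FeatsHandler holds a character's list of feats in the RPG system.
; AddFeat adds only unique feats and calls CallChange when the add succeeds, while RemoveFeat calls it after every removal attempt.
; GetAttackFeats and GetAbilitiesFeats cast the stored feats to the IAttackProvider and IAbilitiesProvider interfaces, exposing them as attack or ability sources.
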(fn `AddFeat`
  (params (AddedFeat :type "/Game/Unreal_Training_Project/Blueprints/RPG_System/BP_Feat Object Reference"))
  (bind _returnvalue (`KismetArrayLibrary.Array_AddUnique` (`self.CharacterFeats`) AddedFeat))
  (if (>= _returnvalue 0)
    (`self.Change`)))

(fn `GetAbilitiesFeats`
  (returns (abilitiesFeats :type "Array of /Game/Unreal_Training_Project/Blueprints/RPG_System/IAbilitiesProvider Interface"))
  (locals (result :type "Array of /Game/Unreal_Training_Project/Blueprints/RPG_System/IAbilitiesProvider Interface"))
  (bind _result (`local.result`))
  (for _array_element (`self.CharacterFeats`)
    (bind _asiabilities_provider (cast `/Game/Unreal_Training_Project/Blueprints/RPG_System/IAbilitiesProvider` _array_element))
    (`KismetArrayLibrary.Array_Add` _result _asiabilities_provider))
  (return _result))

(fn `GetAttackFeats`
  (returns (attackFeats :type "Array of /Game/Unreal_Training_Project/Blueprints/RPG_System/IAttackProvider Interface"))
  (locals (result :type "Array of /Game/Unreal_Training_Project/Blueprints/RPG_System/IAttackProvider Interface"))
  (bind _result (`local.result`))
  (for _array_element (`self.CharacterFeats`)
    (bind _asiattack_provider (cast `/Game/Unreal_Training_Project/Blueprints/RPG_System/IAttackProvider` _array_element))
    (`KismetArrayLibrary.Array_Add` _result _asiattack_provider))
  (return _result))

(fn `RemoveFeat`
  (params (removedFeat :type "/Game/Unreal_Training_Project/Blueprints/RPG_System/BP_Feat Object Reference"))
  (`KismetArrayLibrary.Array_RemoveItem` (`self.CharacterFeats`) removedFeat)
  (`self.Change`))