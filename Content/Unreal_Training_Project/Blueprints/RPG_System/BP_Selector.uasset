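; BP_Selector manages which character is selected in the RPG system, apparently for turn handling.
; It keeps an array of TurnHandlers from added characters, binds to each one's status-change event, and supports removal by index.
; On each addition or status change, CheckSelected looks for a Selected handler, falling back to CheckReady, which promotes a Ready handler to Selected and records its index.
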(fn `AddCharacter`
  (params (`New Character` :type "/Game/Unreal_Training_Project/Blueprints/RPG_System/BP_Character Object Reference"))
  (bind _turnhandler (`/Game/Unreal_Training_Project/Blueprints/RPG_System/BP_Character.TurnHandler` `New Character`))
  (`KismetArrayLibrary.Array_Add` (`self.TurnHandlers`) _turnhandler)
  (`self.CheckSelected`)
  (add `/Game/Unreal_Training_Project/Blueprints/RPG_System/BP_TurnHandler.StatusChange` _turnhandler (`|CreateDelegate` :!event `OnStatusChange`)))

(fn `CheckReady`
  (returns (HasReady :type Boolean))
  (locals (result :type Boolean))
  (for (_array_element _array_index) (`self.TurnHandlers`)
    (bind _returnvalue (`|EnumEquality` (`/Game/Unreal_Training_Project/Blueprints/RPG_System/BP_TurnHandler.Status` _array_element) "Ready"))
    (if _returnvalue
      (set `/Game/Unreal_Training_Project/Blueprints/RPG_System/BP_TurnHandler.Status` "Selected" _array_element)
      (set `self.SelectedIndex` _array_index)
      (return _returnvalue))))

(fn `CheckSelected`
  (returns (HasSelected :type Boolean))
  (for _array_element (`self.TurnHandlers`)
    (bind _returnvalue (`|EnumEquality` (`/Game/Unreal_Training_Project/Blueprints/RPG_System/BP_TurnHandler.Status` _array_element) "Selected"))
    (if _returnvalue
      (set `self.SelectedIndex` 0)
      (return _returnvalue)
      (else
        (bind _hasready (`self.CheckReady` :!label _label))
        (return _hasready))))
  (goto _label))

(fn `GetSelectedIndex`
  (returns (Index :type Integer))
  (for (_array_element _array_index) (`self.TurnHandlers`)
    (if (`|EnumEquality` (`/Game/Unreal_Training_Project/Blueprints/RPG_System/BP_TurnHandler.Status` _array_element) "Selected")
      (return _array_index))))

(fn `OnStatusChange`
  (`self.CheckSelected`))

(fn `RemoveCharacter`
  (params (Index :type Integer))
  (`KismetArrayLibrary.Array_Remove` (`self.TurnHandlers`) Index))