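; BP_Health is an RPG health object that tracks current and maximum HP.
; Max HP derives from base HP plus Constitution bonus times level, and Set fills current HP to it.
; AddHP caps at max and RemoveHP has no floor; both fire CurrentHPChange.
; SetMaxHP adds the entire new max to current HP, and SetConstitutionBonus adjusts both totals through it without storing the new bonus.
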(fn `Add Base HP`
  (params (BaseHPBonusParam :type Integer))
  (set `self.baseHP` (+ (`self.baseHP`) BaseHPBonusParam))
  (set `self.currentHP` (+ (`self.currentHP`) BaseHPBonusParam))
  (`self.Calculate Max Health`))

(fn `AddHP`
  (params (Value :type Integer))
  (bind _output_get (set `self.currentHP` (+ Value (`self.currentHP`))))
  (if (> _output_get (`self.maxHP`))
    (set `self.currentHP` (`self.maxHP`)))
  (`self.CurrentHPChange`))

(fn `Calculate Max Health`
  (returns (MaxHP :type Integer))
  (bind _output_get (set `self.maxHP` (+ (`self.baseHP`) (* (`self.constitutionBonus`) (`self.currentLevel`)))))
  (return _output_get))

(fn `RemoveHP`
  (params (Value :type Integer))
  (locals (deathBorder :type Integer))
  (set `self.currentHP` (- (`self.currentHP`) Value))
  (`self.CurrentHPChange`))

(fn `Set`
  (params (BaseHealthParam :type Integer) (ConstitutionBonusParam :type Integer) (currentLevelParam :type Integer))
  (returns (value :type "/Game/Unreal_Training_Project/Blueprints/RPG_System/BP_Health Object Reference"))
  (set `self.baseHP` BaseHealthParam)
  (set `self.constitutionBonus` ConstitutionBonusParam)
  (set `self.currentLevel` currentLevelParam)
  (bind _maxhp (`self.Calculate Max Health`))
  (set `self.currentHP` _maxhp)
  (return self))

(fn `Set Max HP`
  (params (MaxHealthParam :type Integer))
  (if (!= MaxHealthParam (`self.maxHP`))
    (set `self.currentHP` (+ (- MaxHealthParam 0) (`self.currentHP`)))
    (set `self.maxHP` MaxHealthParam)))

(fn `SetConstitutionBonus`
  (params (ConstitutionBonusParam :type Integer))
  (bind _returnvalue (* (- ConstitutionBonusParam (`self.constitutionBonus`)) (`self.currentLevel`)))
  (set `self.currentHP` (+ _returnvalue (`self.currentHP`)))
  (`self.Set Max HP` (+ _returnvalue (`self.maxHP`))))

(fn `SetCurrentLevel`
  (params (CurrentLevelParam :type Integer))
  (set `self.currentLevel` CurrentLevelParam)
  (`self.Calculate Max Health`))