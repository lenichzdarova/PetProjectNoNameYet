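; BP_PlayerParty manages the player's RPG party: a list of member characters and the index of the active one.
; Adding respects a maximum party size, while removal works by index and leaves the active index unchanged.
; Membership changes fire PartyChanged and selecting an active character fires ActiveCharacterChanged, so other systems can react.
; Getters expose the member list and the active character, with no index validation.
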(fn `AddCharacter`
  (params (Character :type "CharacterData Object Reference"))
  (if (< (`KismetArrayLibrary.Array_Length` (`self.partyMembers`)) (`self.PartyMembersMaxCount`))
    (`KismetArrayLibrary.Array_Add` (`self.partyMembers`) Character)
    (`self.PartyChanged`)))

(fn `GetActiveCharacter`
  (returns (NewParam :type "CharacterData Object Reference"))
  (return (`|GetArrayItem` (`self.partyMembers`) (`self.currentActive`))))

(fn `GetPartyMembers`
  (returns (NewParam :type "Array of CharacterData Object Reference"))
  (return (`self.partyMembers`)))

(fn `RemoveCharacter`
  (params (CharacterIndex :type Integer))
  (`KismetArrayLibrary.Array_Remove` (`self.partyMembers`) CharacterIndex)
  (`self.PartyChanged`))

(fn `SetActiveCharacter`
  (params (`Character index` :type Integer))
  (set `self.currentActive` `Character index`)
  (`self.ActiveCharacterChanged`))