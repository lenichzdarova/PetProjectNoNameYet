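; ForTest is a scratch Blueprint for trying out RPG character object construction and printing the results.
; An unconnected EventGraph chain assembles a BP_Character from profession, feats, effects, abilities and health objects, combining racial abilities and printing max HP.
; The Set function builds Dwarf CharacterData from separate feats, effects, experience and health handlers, then prints its Strength.
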(fn `set`
  (returns (NewParam :type "/Game/Unreal_Training_Project/Blueprints/RPG_System/BP_Character Object Reference"))
  (bind _returnvalue (`|GenericCreateObject` "/Script/Unreal_Training.CharacterData"))
  (bind _returnvalue_2 (`|GenericCreateObject` "/Script/Unreal_Training.FeatsHandler"))
  (bind _returnvalue_3 (`|GenericCreateObject` "/Script/Unreal_Training.EffectsHandler"))
  (bind _returnvalue_4 (`|GenericCreateObject` "/Script/Unreal_Training.ExperienceHandler"))
  (bind _returnvalue_5 (`|GenericCreateObject` "/Script/Unreal_Training.HealthHandler"))
  (`CharacterData.Set` _returnvalue "Dwarf" (`self.portrait`) _returnvalue_2 _returnvalue_3 (`BaseDataProvidersLibrary.GetBaseRaceAbilities` "Dwarf") _returnvalue_4 _returnvalue_5)
  (bind _returnvalue_6 (`CharacterData.GetAbilities` _returnvalue))
  (`KismetSystemLibrary.PrintString` null (`KismetStringLibrary.Conv_IntToString` (`Abilities.strength` _returnvalue_6))))