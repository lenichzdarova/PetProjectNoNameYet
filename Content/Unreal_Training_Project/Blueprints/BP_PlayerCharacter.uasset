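; First-person player character that handles looking, moving and jumping through Enhanced Input, adding its mapping context on BeginPlay.
; Look input turns controller yaw and pitches the camera directly, without clamping.
; Movement offsets the actor along control-rotation axes by MoveSpeed, without sweep or delta-time scaling, bypassing character movement.
; Party panel creation, random-member damage test and AddMovementInput logic are disconnected, and LookUp and LookRight are not called here.
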(event `self.ReceiveBeginPlay`
  (bind _asplayer_controller (cast `PlayerController` (`self.GetController`)))
  (message `EnhancedInputSubsystemInterface.AddMappingContext` (pcsubsystem `EnhancedInputLocalPlayerSubsystem` _asplayer_controller) "/Game/Unreal_Training_Project/Blueprints/Inputs/IAM_FirstPerson.IAM_FirstPerson" 0 (struct))
  (bind _returnvalue (`GameplayStatics.GetCurrentLevelName` true)))

(event `Key|F`
  (params (Key :type "Key Structure"))
  ;[1 1 1] Only for test
)

(event `EnhancedInput|/Game/Unreal_Training_Project/Blueprints/Inputs/IA_Look`
  (params (ActionValue :type "Vector2D Structure") (ElapsedSeconds :type "Float (double-precision)") (TriggeredSeconds :type "Float (double-precision)") (InputAction :type "InputAction Object Reference" :default "/Game/Unreal_Training_Project/Blueprints/Inputs/IA_Look.IA_Look"))
  (:`Triggered`
    (`self.LookInputHandle` (`KismetMathLibrary.MakeVector2D` ActionValue_X ActionValue_Y))))

(event `EnhancedInput|/Game/Unreal_Training_Project/Blueprints/Inputs/IA_Move`
  (params (ActionValue :type "Vector2D Structure") (ElapsedSeconds :type "Float (double-precision)") (TriggeredSeconds :type "Float (double-precision)") (InputAction :type "InputAction Object Reference" :default "/Game/Unreal_Training_Project/Blueprints/Inputs/IA_Move.IA_Move"))
  (:`Triggered`
    (`self.MoveInputHandle` (`KismetMathLibrary.MakeVector2D` ActionValue_X ActionValue_Y))))

(event `EnhancedInput|/Game/Unreal_Training_Project/Blueprints/Inputs/IA_Jump`
  (params (ActionValue :type Boolean) (ElapsedSeconds :type "Float (double-precision)") (TriggeredSeconds :type "Float (double-precision)") (InputAction :type "InputAction Object Reference" :default "/Game/Unreal_Training_Project/Blueprints/Inputs/IA_Jump.IA_Jump"))
  (:`Triggered`
    (`self.Jump`)))

(fn `Look RIght`
  (params (InputValue :type "Float (double-precision)"))
  (`self.AddControllerYawInput` InputValue))

(fn `LookInputHandle`
  (params (InputValue :type "Vector2D Structure"))
  (bind (_returnvalue_roll _returnvalue_pitch _returnvalue_yaw) (`KismetMathLibrary.BreakRotator` (`SceneComponent.K2_GetComponentRotation` (`self.Camera`))))
  (`self.AddControllerYawInput` InputValue_X)
  (`SceneComponent.K2_SetWorldRotation` (`self.Camera`) (`KismetMathLibrary.MakeRotator` 0.0 (+ InputValue_Y _returnvalue_pitch) _returnvalue_yaw) false false))

(fn `LookUp`
  (params (InputValue :type "Float (double-precision)"))
  (bind (_returnvalue_roll _returnvalue_pitch _returnvalue_yaw) (`KismetMathLibrary.BreakRotator` (`self.GetControlRotation`)))
  (bind (_returnvalue_roll_2 _returnvalue_pitch_2) (`KismetMathLibrary.BreakRotator` (`SceneComponent.K2_GetComponentRotation` (`self.Camera`))))
  (`SceneComponent.K2_SetWorldRotation` (`self.Camera`) (`KismetMathLibrary.MakeRotator` 0.0 (+ InputValue _returnvalue_pitch_2) _returnvalue_yaw) false false))

(fn `MoveInputHandle`
  (params (InputValue :type "Vector2D Structure"))
  (locals (NewLocalVar :type Boolean))
  (bind _returnvalue (`self.GetControlRotation`))
  (`self.K2_AddActorWorldOffset` (* (+ (* InputValue_X (`KismetMathLibrary.GetForwardVector` _returnvalue)) (* (`KismetMathLibrary.GetRightVector` _returnvalue) InputValue_Y)) (`self.MoveSpeed`))))

(fn `UserConstructionScript`)